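; Player character Blueprint providing turn, look, camera-relative movement, free look, pose/move state and walk-speed functions.
; Free look unlocks controller yaw while movement keeps the saved heading; on release a timeline lerps control rotation back by the shortest path, then relocks yaw.
; Move state resolves from input flags through an overriding sequence, with aim above walk above run.
; Tick broadcasts only when the character starts or stops moving.
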(event `self.ReceiveTick`
  (params (DeltaSeconds :type "Float (single-precision)"))
  (bind _returnvalue (> (`KismetMathLibrary.VSizeSquared` (`self.GetVelocity`)) 0.0))
  ; 단순비교는 tick 에서 해도 돼
  (if (!= (`self.bIsMovingNow`) _returnvalue)
    (bind _output_get (set `self.bIsMovingNow` _returnvalue))
    ; 나 신호 바뀌었어
    (`self.OnMovementStateChanged` _output_get)))

(event `OnFreeLookEnded`
  (bind (_direction _alpha) (`Timeline|Timeline` :!via `PlayFromStart`)
    (:`Update`
      (`Controller.SetControlRotation` (`self.GetController`) (`KismetMathLibrary.RLerp` (`self.FreeLookEndRotation`) (`self.FreeLookStartRotation`) _alpha true)))
    (:`Finished`
      (set `self.bUseControllerRotationYaw` true))))

(fn `EvaluateMoveState`
  ; 이 방식으로할거다
  (`|ExecutionSequence`
    (:`then_0`
      (set `self.CurrentMoveState` "NewEnumerator1"))
    (:`then_1`
      (if (`self.bIsRunPressed`)
        (set `self.CurrentMoveState` "NewEnumerator2")))
    (:`then_2`
      (if (`self.bIsWalkPressed`)
        (set `self.CurrentMoveState` "NewEnumerator0")))
    (:`then_3`
      (if (`self.bIsAimPressed`)
        (set `self.CurrentMoveState` "NewEnumerator3")))))

(fn `FreeLook`
  (params (bIsPressed :type Boolean))
  (bind _returnvalue (`self.GetControlRotation`))
  (if bIsPressed
    ; FreeLook 시작 로테이션
    (set `self.FreeLookStartRotation` _returnvalue)
    (set `self.bUseControllerRotationYaw` false)
    (else
      ; FreeLook 끝났을 때 회전
      (set `self.FreeLookEndRotation` _returnvalue)
      ; 호출부
      (`self.OnFreeLookEnded`))))

(fn `GetMoveRotation`
  (returns (Result :type "Rotator Structure"))
  (locals (ResultRotator :type "Rotator Structure"))
  (return (`KismetMathLibrary.SelectRotator` (`/Game/Blueprints/Util/MathUtils.GetYawOnlyRotation` (`self.GetControlRotation`)) (`/Game/Blueprints/Util/MathUtils.GetYawOnlyRotation` (`self.FreeLookStartRotation`)) (`self.bUseControllerRotationYaw`))))

(fn `InputLookUp`
  (params (`Y Axis` :type "Float (double-precision)"))
  (`self.AddControllerPitchInput` `Y Axis`))

(fn `InputTurn`
  (params (`X Axis` :type "Float (double-precision)"))
  (`self.AddControllerYawInput` `X Axis`))

(fn `Move`
  (params (bIsForward :type Boolean) (`Axis Value` :type "Float (double-precision)"))
  (locals (NewLocalVar :type "AudioMaterialButton Object Reference"))
  (bind _result (`self.GetMoveRotation`))
  (if bIsForward
    (`self.AddMovementInput` (`KismetMathLibrary.GetForwardVector` _result) (`local.Axis Value`))
    (else
      (`self.AddMovementInput` (`KismetMathLibrary.GetRightVector` _result) (`local.Axis Value`)))))

(fn `SetMaxWalkSpeed`
  (params (NewSpeed :type "Float (double-precision)"))
  (set `CharacterMovementComponent.MaxWalkSpeed` NewSpeed (`self.CharacterMovement`)))

(fn `UpdateMoveState`
  (params (NewState :type "/Game/Blueprints/Datas/Enum/E_MoveState Enum" :default "NewEnumerator0"))
  (set `self.CurrentMoveState` NewState))

(fn `UpdatePoseState`
  (params (NewState :type "/Game/Blueprints/Datas/Enum/E_PoseState Enum" :default "NewEnumerator0"))
  (set `self.CurrentPoseState` NewState))

(fn `UserConstructionScript`)